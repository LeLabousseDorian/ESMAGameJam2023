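; BP_AC_Life is a life component that tracks its owning actor's hit points.
; TakeDamage only has an effect once the owner's X scale reaches a minimum size, and larger owners lose less HP because damage is divided by twice that scale.
; It then broadcasts OnTakeDamage with the unscaled damage and remaining HP, followed by OnDeath when HP reaches zero or below.
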(fn `TakeDamage`
  (params (Damage :type "Float (double-precision)"))
  (bind _returnvalue_x (`KismetMathLibrary.BreakVector` (`Actor.GetActorScale3D` (`self.GetOwner`))))
  (if (>= _returnvalue_x 3.0)
    (bind _output_get (set `self.CurrentHp` (- (`self.CurrentHp`) (* Damage (/ (/ 1.0 _returnvalue_x) 2.0)))))
    (`self.OnTakeDamage` (`local.Damage`) _output_get)
    (if (<= (`self.CurrentHp`) 0.0)
      (`self.OnDeath`))))