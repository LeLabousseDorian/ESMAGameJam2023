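; BP_DamageBox is a hazard volume that deals periodic damage to a BP_Character inside its Hitbox.
; Begin and end overlap events store and clear a single Player reference.
; A looping timer, started on BeginPlay at TickRate, applies Damage through that character's Life while the reference is valid.
; The timer runs independently of overlaps, so entering does not deal damage immediately.
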(event `self.ReceiveBeginPlay`
  (`KismetSystemLibrary.K2_SetTimerDelegate` (delegate `DamagePlayer`) (`self.TickRate`) true))

(event `DamagePlayer`
  (bind _player (`self.Player`))
  (`/Engine/EditorBlueprintResources/StandardMacros.IsValid` _player
    (:`Is Valid`
      (`/Game/Blueprint/Components/BP_AC_Life.TakeDamage` (`/Game/Blueprint/Characters/Player/BP_Character.Life` _player) (`self.Damage`)))))

(event `self.hitbox.OnComponentBeginOverlap`
  (params (OverlappedComponent :type "PrimitiveComponent Object Reference") (OtherActor :type "Actor Object Reference") (OtherComp :type "PrimitiveComponent Object Reference") (OtherBodyIndex :type Integer) (bFromSweep :type Boolean) (SweepResult :type "HitResult Structure (by ref)"))
  (bind _asbp_character (cast `/Game/Blueprint/Characters/Player/BP_Character` OtherActor))
  (set `self.Player` _asbp_character))

(event `self.hitbox.OnComponentEndOverlap`
  (params (OverlappedComponent :type "PrimitiveComponent Object Reference") (OtherActor :type "Actor Object Reference") (OtherComp :type "PrimitiveComponent Object Reference") (OtherBodyIndex :type Integer))
  (cast `/Game/Blueprint/Characters/Player/BP_Character` OtherActor)
  (set `self.Player` null))

(fn `UserConstructionScript`)