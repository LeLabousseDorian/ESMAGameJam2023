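; Slime enemy character that detects the player and deals melee damage through a timed hitbox.
; A detection sphere sets or clears the Player blackboard key, and Attack toggles bAttacking for the AI.
; Attack briefly enables and shows the box after a delay, damaging each character once per swing.
; StarShoot launches the physics-simulated capsule upward and toward PlayerLocation with a hit sound, and landing turns physics off.
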(event `self.SphereDetection.OnComponentBeginOverlap`
  (params (OverlappedComponent :type "PrimitiveComponent Object Reference") (OtherActor :type "Actor Object Reference") (OtherComp :type "PrimitiveComponent Object Reference") (OtherBodyIndex :type Integer) (bFromSweep :type Boolean) (SweepResult :type "HitResult Structure (by ref)"))
  ;[1 1 1] Overlap Start/End Player
  (bind _asbp_character (cast `/Game/Blueprint/Characters/Player/BP_Character` OtherActor))
  (`BlackboardComponent.SetValueAsObject` (`AIBlueprintHelperLibrary.GetBlackboard` null) "Player" _asbp_character))

(event `self.SphereDetection.OnComponentEndOverlap`
  (params (OverlappedComponent :type "PrimitiveComponent Object Reference") (OtherActor :type "Actor Object Reference") (OtherComp :type "PrimitiveComponent Object Reference") (OtherBodyIndex :type Integer))
  ;[1 1 1] Overlap Start/End Player
  (cast `/Game/Blueprint/Characters/Player/BP_Character` OtherActor)
  (`BlackboardComponent.SetValueAsObject` (`AIBlueprintHelperLibrary.GetBlackboard` null) "Player" null))

(event `self.Box.OnComponentBeginOverlap`
  (params (OverlappedComponent :type "PrimitiveComponent Object Reference") (OtherActor :type "Actor Object Reference") (OtherComp :type "PrimitiveComponent Object Reference") (OtherBodyIndex :type Integer) (bFromSweep :type Boolean) (SweepResult :type "HitResult Structure (by ref)"))
  ;[1 1 1] Hitbox Overlap
  (if (not (`self.AlreadyHit` OtherActor))
    (bind _asbp_character (cast `/Game/Blueprint/Characters/Player/BP_Character` OtherActor))
    (`/Game/Blueprint/Components/BP_AC_Life.TakeDamage` (`/Game/Blueprint/Characters/Player/BP_Character.Life` _asbp_character) (`self.Damage`))
    (`KismetArrayLibrary.Array_AddUnique` (`self.ActorAlreadyHit`) _asbp_character)))

(event `Attack`
  ;[1 1 1] Attack
  (if (not (`self.bAttacking`))
    (`BlackboardComponent.SetValueAsBool` (`AIBlueprintHelperLibrary.GetBlackboard` null) "bAttacking" true)
    (set `self.bAttacking` true)
    (`KismetSystemLibrary.Delay` 0.5)
    (`self.HitboxUp`)
    (`KismetSystemLibrary.Delay` 0.5)
    (`self.StopAttack`)))

(event `StopAttack`
  ;[1 1 1] Stop Attack
  (if (`self.bAttacking`)
    (set `self.bAttacking` false)
    (`BlackboardComponent.SetValueAsBool` (`AIBlueprintHelperLibrary.GetBlackboard` null) "bAttacking" false)
    (`self.HitboxDown`)
    (`KismetArrayLibrary.Array_Clear` (`self.ActorAlreadyHit`))))

(event `StarShoot`
  (params (PlayerLocation :type "Vector Structure") (Size :type "Float (double-precision)") (Velocity :type "Float (double-precision)"))
  (bind (_returnvalue_x _returnvalue_y _returnvalue_z) (`KismetMathLibrary.BreakVector` (`self.K2_GetActorLocation`)))
  (bind _capsulecomponent (`self.CapsuleComponent`))
  (bind (_returnvalue_x_2 _returnvalue_y_2) (`KismetMathLibrary.BreakVector` (* (`KismetMathLibrary.MakeVector` (- PlayerLocation_X _returnvalue_x) (- PlayerLocation_Y _returnvalue_y) (- PlayerLocation_Z _returnvalue_z)) 10000.0)))
  (bind (_returnvalue_x_3 _returnvalue_y_3) (`KismetMathLibrary.BreakVector` (`KismetMathLibrary.MakeVector` _returnvalue_x_2 _returnvalue_y_2)))
  (`PrimitiveComponent.SetSimulatePhysics` _capsulecomponent true)
  (`PrimitiveComponent.AddImpulse` _capsulecomponent (`KismetMathLibrary.MakeVector` _returnvalue_x_3 _returnvalue_y_3 10000.0) "pelvis" false)
  (`FMODBlueprintStatics.PlayEventAttached` "/Game/FMOD/Events/HitHard.HitHard" (`self.CapsuleComponent`) "None" (0.0 0.0 0.0) "KeepRelativeOffset"))

(event `self.OnLanded`
  (params (Hit :type "HitResult Structure (by ref)"))
  (`PrimitiveComponent.SetSimulatePhysics` (`self.CapsuleComponent`) false))

(fn `AlreadyHit`
  (params (Actorhit :type "Actor Object Reference"))
  (returns (bAlreadyHit :type Boolean))
  (locals (bLoc_AlreadyHit :type Boolean))
  (for _array_element (`self.ActorAlreadyHit`)
    (bind _output_get (set `local.bLoc_AlreadyHit` (== _array_element Actorhit)))
    (if _output_get
      (break)))
  (return (`local.bLoc_AlreadyHit`)))

(fn `HitboxDown`
  (bind _box (`self.Box`))
  (`PrimitiveComponent.SetCollisionEnabled` _box "NoCollision")
  (`SceneComponent.SetHiddenInGame` _box true false)
  (`SceneComponent.SetVisibility` _box false false))

(fn `HitboxUp`
  (bind _box (`self.Box`))
  (`PrimitiveComponent.SetCollisionEnabled` _box "QueryOnly")
  (`SceneComponent.SetHiddenInGame` _box false false)
  (`SceneComponent.SetVisibility` _box true false))

(fn `UserConstructionScript`)