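; Base slime enemy that chases or tracks the player through AI, deals contact damage and can be launched to its death.
; A detection sphere sets and clears the Player blackboard key on overlap.
; Hitbox overlaps damage the player's Life component, with collision briefly disabled as a cooldown.
; StarShoot turns on mesh physics, launches it up and away from the player scaled by size and velocity, plays a hit sound, then destroys the actor.
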(event `self.SphereDetection.OnComponentBeginOverlap`
  (params (OverlappedComponent :type "PrimitiveComponent Object Reference") (OtherActor :type "Actor Object Reference") (OtherComp :type "PrimitiveComponent Object Reference") (OtherBodyIndex :type Integer) (bFromSweep :type Boolean) (SweepResult :type "HitResult Structure (by ref)"))
  ;[1 1 1] Overlap Start/End Player
  (bind _asbp_character (cast `/Game/Blueprint/Characters/Player/BP_Character` OtherActor))
  (`BlackboardComponent.SetValueAsObject` (`AIBlueprintHelperLibrary.GetBlackboard` null) "Player" _asbp_character))

(event `self.SphereDetection.OnComponentEndOverlap`
  (params (OverlappedComponent :type "PrimitiveComponent Object Reference") (OtherActor :type "Actor Object Reference") (OtherComp :type "PrimitiveComponent Object Reference") (OtherBodyIndex :type Integer))
  (bind _returnvalue (`AIBlueprintHelperLibrary.GetBlackboard` null))
  ;[1 1 1] Overlap Start/End Player
  (cast `/Game/Blueprint/Characters/Player/BP_Character` OtherActor)
  (`/Engine/EditorBlueprintResources/StandardMacros.IsValid` _returnvalue
    (:`Is Valid`
      (`BlackboardComponent.SetValueAsObject` _returnvalue "Player" null))))

(event `self.Hitbox.OnComponentBeginOverlap`
  (params (OverlappedComponent :type "PrimitiveComponent Object Reference") (OtherActor :type "Actor Object Reference") (OtherComp :type "PrimitiveComponent Object Reference") (OtherBodyIndex :type Integer) (bFromSweep :type Boolean) (SweepResult :type "HitResult Structure (by ref)"))
  ;[1 1 1] Damage player
  (`self.DealDamageToPlayer` OtherActor)
  (`KismetSystemLibrary.Delay` 0.5)
  (`PrimitiveComponent.SetCollisionEnabled` (`self.Hitbox`) "QueryOnly"))

(event `StarShoot`
  (params (PlayerLocation :type "Vector Structure") (Size :type "Float (double-precision)") (Velocity :type "Float (double-precision)"))
  (bind (_returnvalue_x _returnvalue_y _returnvalue_z) (`KismetMathLibrary.BreakVector` (`self.K2_GetActorLocation`)))
  (bind _mesh (`self.Mesh`))
  (bind (_returnvalue_x_2 _returnvalue_y_2) (`KismetMathLibrary.BreakVector` (* (`KismetMathLibrary.MakeVector` (- PlayerLocation_X _returnvalue_x) (- PlayerLocation_Y _returnvalue_y) (- PlayerLocation_Z _returnvalue_z)) (`self.StarShootBaseForce`))))
  (bind (_returnvalue_x_3 _returnvalue_y_3) (`KismetMathLibrary.BreakVector` (`KismetMathLibrary.MakeVector` _returnvalue_x_2 _returnvalue_y_2)))
  (bind (_returnvalue_x_4 _returnvalue_y_4) (`KismetMathLibrary.BreakVector` (* (* (`KismetMathLibrary.MakeVector` _returnvalue_x_3 _returnvalue_y_3) (* (/ Size 3.0) (/ (`KismetMathLibrary.FClamp` (- Velocity 600.0) 300.0 3000.0) 300.0))) -1.0)))
  ;[1 1 1] StarShoot
  (`SkeletalMeshComponent.SetAllBodiesSimulatePhysics` _mesh true)
  (`PrimitiveComponent.SetSimulatePhysics` _mesh true)
  (`PrimitiveComponent.WakeAllRigidBodies` _mesh)
  (`PrimitiveComponent.AddImpulse` _mesh (`KismetMathLibrary.MakeVector` _returnvalue_x_4 _returnvalue_y_4 1000.0) "pelvis" false)
  (`PrimitiveComponent.SetCollisionEnabled` (`self.CapsuleComponent`) "NoCollision")
  (`FMODBlueprintStatics.PlayEventAttached` "/Game/FMOD/Events/HitHard.HitHard" (`self.CapsuleComponent`) "pelvis" (0.0 0.0 0.0) "KeepRelativeOffset")
  (`KismetSystemLibrary.Delay` 5.0)
  (`self.K2_DestroyActor`))

(fn `DealDamageToPlayer`
  (params (Actor :type "Object Object Reference"))
  (bind _asbp_character (cast `/Game/Blueprint/Characters/Player/BP_Character` Actor))
  (`/Game/Blueprint/Components/BP_AC_Life.TakeDamage` (`/Game/Blueprint/Characters/Player/BP_Character.Life` _asbp_character) (`self.Damage`))
  (`PrimitiveComponent.SetCollisionEnabled` (`self.Hitbox`) "NoCollision"))

(fn `UserConstructionScript`)