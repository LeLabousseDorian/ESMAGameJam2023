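; BP_NewHammer is a pickup that grants the player character the glitch hammer.
; When a BP_Character overlaps its Hitbox, it sets that character's GlitchHammer flag and copies three material slots from its own Hammer mesh onto the character's Hammer.
; It then plays the Marteau_glitch sound in 2D and destroys itself.
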(event `self.Hitbox.OnComponentBeginOverlap`
  (params (OverlappedComponent :type "PrimitiveComponent Object Reference") (OtherActor :type "Actor Object Reference") (OtherComp :type "PrimitiveComponent Object Reference") (OtherBodyIndex :type Integer) (bFromSweep :type Boolean) (SweepResult :type "HitResult Structure (by ref)"))
  (bind _returnvalue (`MeshComponent.GetMaterials` (`self.Hammer`)))
  (bind _asbp_character (cast `/Game/Blueprint/Characters/Player/BP_Character` OtherActor))
  (set `/Game/Blueprint/Characters/Player/BP_Character.bGlitchHammer` true _asbp_character)
  (bind _hammer (`/Game/Blueprint/Characters/Player/BP_Character.Hammer` _asbp_character))
  (`PrimitiveComponent.SetMaterial` _hammer 0 (`|GetArrayItem` _returnvalue))
  (`PrimitiveComponent.SetMaterial` _hammer 1 (`|GetArrayItem` _returnvalue 1))
  (`PrimitiveComponent.SetMaterial` _hammer 2 (`|GetArrayItem` _returnvalue 2))
  (`GameplayStatics.PlaySound2D` "/Game/SFX/Marteau_glitch.Marteau_glitch" 1.0 1.0 0.0 null null)
  (`self.K2_DestroyActor`))

(fn `UserConstructionScript`)