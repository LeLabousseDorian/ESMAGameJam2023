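; BP_Star is a collectible pickup in the coins set that spins in the world.
; It gives the static mesh a random yaw on BeginPlay, then adds a fixed yaw step every Tick, so rotation speed follows frame rate.
; When a BP_Character overlaps the sphere, it calls GetCoins on the character, plays the attached Pickup audio event and destroys itself.
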(event `self.ReceiveBeginPlay`
  ;[1 1 1] Random Start Rotation
  (`SceneComponent.K2_SetWorldRotation` (`self.StaticMesh`) (`KismetMathLibrary.MakeRotator` 0.0 0.0 (`KismetMathLibrary.RandomFloatInRange` 0.0 360.0)) false false))

(event `self.ReceiveTick`
  (params (DeltaSeconds :type "Float (single-precision)"))
  ;[1 1 1] Rotation Anim
  (`SceneComponent.K2_AddWorldRotation` (`self.StaticMesh`) (struct :`Yaw` 1.0) false false))

(event `self.Sphere.OnComponentBeginOverlap`
  (params (OverlappedComponent :type "PrimitiveComponent Object Reference") (OtherActor :type "Actor Object Reference") (OtherComp :type "PrimitiveComponent Object Reference") (OtherBodyIndex :type Integer) (bFromSweep :type Boolean) (SweepResult :type "HitResult Structure (by ref)"))
  ;[1 1 1] Add Coins
  (bind _asbp_character (cast `/Game/Blueprint/Characters/Player/BP_Character` OtherActor))
  (`/Game/Blueprint/Characters/Player/BP_Character.GetCoins` _asbp_character)
  (`FMODBlueprintStatics.PlayEventAttached` "/Game/FMOD/Events/Pickup.Pickup" (`self.StaticMesh`) "None" (0.0 0.0 0.0) "KeepRelativeOffset")
  (`self.K2_DestroyActor`))

(fn `UserConstructionScript`)