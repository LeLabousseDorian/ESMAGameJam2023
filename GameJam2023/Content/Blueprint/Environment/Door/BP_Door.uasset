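; BP_Door is a coin-gated door that rises when a BP_Character with at least 100 coins overlaps its Hitbox.
; The overlap only checks the coin count, without deducting it, then calls OpenDoor, which a DoOnce limits to a single run.
; The Open timeline serves as an update tick, each step using VInterpTo to nudge the Door upward from its current relative location rather than toward a fixed end point.
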(event `self.Hitbox.OnComponentBeginOverlap`
  (params (OverlappedComponent :type "PrimitiveComponent Object Reference") (OtherActor :type "Actor Object Reference") (OtherComp :type "PrimitiveComponent Object Reference") (OtherBodyIndex :type Integer) (bFromSweep :type Boolean) (SweepResult :type "HitResult Structure (by ref)"))
  ;[1 1 1] Player collide with door
  (bind _asbp_character (cast `/Game/Blueprint/Characters/Player/BP_Character` OtherActor))
  (if (>= (`/Game/Blueprint/Characters/Player/BP_Character.Coins` _asbp_character) 100)
    (`self.OpenDoor`)))

(event `OpenDoor`
  (bind _relativelocation (`SceneComponent.RelativeLocation` (`self.Door`)))
  (`/Engine/EditorBlueprintResources/StandardMacros.DoOnce` false
    (:`Completed`
      (bind (_direction _deltatime) (`Timeline|Open` :!via `PlayFromStart`)
        (:`Update`
          (`SceneComponent.K2_SetRelativeLocation` (`self.Door`) (`KismetMathLibrary.VInterpTo` _relativelocation (+ _relativelocation (0.0 0.0 300.0)) _deltatime 0.07) false false))))))

(fn `UserConstructionScript`)