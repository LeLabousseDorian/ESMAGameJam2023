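; BP_Rock is an environment rock actor that gets knocked away from the player and removed.
; Its Destroy event enables physics simulation on the Rock component and applies a large horizontal impulse pointing away from the supplied player location.
; After a brief delay, the actor destroys itself.
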(event `Destroy`
  (params (PlayerLoc :type "Vector Structure"))
  (bind (_returnvalue_x _returnvalue_y) (`KismetMathLibrary.BreakVector` (`self.K2_GetActorLocation`)))
  (`PrimitiveComponent.SetSimulatePhysics` (`self.Rock`) true)
  (`PrimitiveComponent.AddImpulse` (`self.Rock`) (* (* (`KismetMathLibrary.Normal` (`KismetMathLibrary.MakeVector` (- PlayerLoc_X _returnvalue_x) (- PlayerLoc_Y _returnvalue_y) 0.0) 0.01) -1.0) 1000000.0) "None" false)
  (`KismetSystemLibrary.Delay` 0.2)
  (`self.K2_DestroyActor`))

(fn `UserConstructionScript`)